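; Actor component that supports flying movement for AI Characters.
; On BeginPlay it caches the owning Character and its capsule and sets CharacterMovement gravity scale to zero, printing an error if the owner is not a Character.
; When ForbidActorPitchingAndRolling is enabled, Tick resets any capsule pitch or roll to zero while keeping yaw, so the actor stays upright.
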(event `self.ReceiveBeginPlay`
  ;[1 1 1] Initialize
  (`self.init`))

(event `self.ReceiveTick`
  (params (DeltaSeconds :type "Float (single-precision)"))
  (bind (_returnvalue_roll _returnvalue_pitch _returnvalue_yaw) (`KismetMathLibrary.BreakRotator` (`SceneComponent.K2_GetComponentRotation` (`self.capsuleComponent`))))
  ;[1 1 1] Forbid pitching & rolling
  (if (`self.forbidActorPitchingAndRolling?`)
    (if (or (!= _returnvalue_roll 0.0) (!= _returnvalue_pitch 0.0))
      (`SceneComponent.K2_SetWorldRotation` (`self.capsuleComponent`) (`KismetMathLibrary.MakeRotator` 0.0 0.0 _returnvalue_yaw) false false) ; Reset pitch and roll
    )))

(fn `init`
  ;[1 1 1] Save references
  (bind _ascharacter (cast `Character` (`self.GetOwner`))
    (:`then`
      (bind _output_get (set `self.OwningChracterRef` _ascharacter))
      (set `self.capsuleComponent` (`Character.CapsuleComponent` _output_get))
      ;[1 1 1] Disable gravity
      (set `CharacterMovementComponent.GravityScale` 0.0 (`Character.CharacterMovement` (`self.OwningChracterRef`))))
    (:`CastFailed`
      (`KismetSystemLibrary.PrintString` "ERROR: PhysicsMoveToParameters component only works with CHARACTERS."))))