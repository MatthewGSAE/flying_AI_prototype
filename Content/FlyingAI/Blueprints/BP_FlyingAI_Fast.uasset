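; BP_FlyingAI_Fast is a flying AI enemy that targets the player and shoots on sight.
; On BeginPlay it hands its behavior tree and the player pawn to its My_AIC controller.
; When PawnSensing sees the third-person character, it snaps its rotation toward that character and spawns a projectile at Arrow1.
; A CanShoot flag and ShootTimer delay throttle the fire rate.
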(event `self.ReceiveBeginPlay`
  ;[1 1 1] Setup the AI Controller with the Target Pawn and the Behavior Tree to use
  (bind _asmy_aic (cast `/Game/FlyingAI/AI/My_AIC` (`AIBlueprintHelperLibrary.GetAIController` self)))
  (`/Game/FlyingAI/AI/My_AIC.Setup AIC` _asmy_aic (`self.BT`) (`GameplayStatics.GetPlayerPawn` 0)))

(event `self.PawnSensing.OnSeePawn`
  (params (Pawn :type "Pawn Object Reference"))
  ;[1 1 1] Shooting
  (bind _asbp_third_person_character (cast `/Game/ThirdPerson/Blueprints/BP_ThirdPersonCharacter` Pawn))
  (`self.K2_SetActorRotation` (`KismetMathLibrary.FindRelativeLookAtRotation` (`KismetMathLibrary.Conv_VectorToTransform` (`self.K2_GetActorLocation`)) (`self.K2_GetActorLocation` _asbp_third_person_character)))
  (if (`self.CanShoot`)
    (`|SpawnActorFromClass` "/Game/FirstPerson/Blueprints/BP_FirstPersonProjectile.BP_FirstPersonProjectile_C" (`SceneComponent.K2_GetComponentToWorld` (`self.Arrow1`)) "Undefined" "MultiplyWithRoot" null null)
    (set `self.CanShoot` false)
    (`KismetSystemLibrary.Delay` (`self.ShootTimer`))
    (set `self.CanShoot` true)))

(fn `UserConstructionScript`)